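; BP_Mole is a whack-a-mole target that awards points when hit.
; A Timeline moves it relative to its BeginPlay location and clears IsMoleActive when finished, with TimelinePLay as the event that starts it from the beginning.
; A BP_Mallet overlap on an active mole plays a honk at world origin, adds points through WhackAMoleManager, then sets the Timeline's time and resumes it.
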(event Custom|TimelinePLay
  (bind _position (Timeline|Timeline PlayFromStart)
    (:Update
      (Transformation|SetActorLocation (+ (Variables|Default|GetTarget%20Location) _position) true false))
    (:Finished
      (Variables|Default|SetisMoleActive false))))

(event EventBeginPlay
  (Variables|Default|SetTarget%20Location (Transformation|GetActorLocation)))

(event Collision|EventActorBeginOverlap
  (params (OtherActor :type Actor%20Object%20Reference))
  (Utilities|Casting|CastToBP_Mallet OtherActor)
  (if (Variables|Default|GetisMoleActive)
    (Audio|PlaySoundatLocation "/Game/Game/Audio/honk.honk" "0, 0, 0" "0, 0, 0" 1.0 1.0 0.0 0 0 0 0)
    (Default|AddPoints (Variables|Default|GetWhackAMoleManager) 5)
    (Utilities|FlowControl|Sequence
      (:then_0
        (bind _position (Timeline|Timeline SetNewTime)
          (:Update
            (Transformation|SetActorLocation (+ (Variables|Default|GetTarget%20Location) _position) true false))
          (:Finished
            (Variables|Default|SetisMoleActive false))))
      (:then_1
        (Timeline|Timeline Play)))))

(event EventTick
  (params (DeltaSeconds :type Float%20%28single-precision%29)))

(fn ConstructionScript)